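; Door actor that slides between its placed location and that location offset by MoveLimit.
; SetIsOpen sets the target state, resets the move timer and records the current location as the new start, so mid-move reversals don't jump.
; Tick advances the timer, capped at MoveTime, and linearly interpolates the actor's location without sweep.
; Every move takes the full MoveTime, even from a partly open position.
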(event EventBeginPlay
  (bind _output_get (Variables|Default|SetInitialLocation (Transformation|GetActorLocation)))
  (bind _output_get_2 (Variables|Default|SetCloseStartLocation _output_get))
  (Variables|Default|SetOpenStartLocation _output_get_2))

(event EventTick
  (params (DeltaSeconds :type Float%20%28single-precision%29))
  (CallFunction|AddAlpha DeltaSeconds)
  (if (Variables|Default|GetIsOpen)
    (Transformation|SetActorLocation (Math|Vector|Lerp(Vector) (Variables|Default|GetOpenStartLocation) (+ (Variables|Default|GetMoveLimit) (Variables|Default|GetInitialLocation)) (CallFunction|GetAlpha)) false false)
    (else
      (Transformation|SetActorLocation (Math|Vector|Lerp(Vector) (Variables|Default|GetCloseStartLocation) (Variables|Default|GetInitialLocation) (CallFunction|GetAlpha)) false false))))

(fn ConstructionScript)

(fn AddAlpha
  (params (DeltaTime :type Float%20%28double-precision%29))
  (bind _output_get (Variables|Default|SetCurrentMoveTime (+ DeltaTime (Variables|Default|GetCurrentMoveTime))))
  (if (> _output_get (Variables|Default|GetMoveTime))
    (Variables|Default|SetCurrentMoveTime (Variables|Default|GetMoveTime))))

(fn SetIsOpen
  (params (IsOpen :type Boolean))
  (bind _returnvalue (Transformation|GetActorLocation))
  (Variables|Default|SetCurrentMoveTime 0.0)
  (bind _output_get (Variables|Default|SetIsOpen IsOpen))
  (if _output_get
    (Variables|Default|SetOpenStartLocation _returnvalue)
    (else
      (Variables|Default|SetCloseStartLocation _returnvalue))))

(fn GetAlpha
  (return (/ (Variables|Default|GetCurrentMoveTime) (Variables|Default|GetMoveTime))))