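; BP_Dummy is a moving dummy actor that slides back and forth and prints a debug "Hello" when hit by BP_FirstPersonProjectile.
; Tick times each leg against MoveTime, pauses through a Delay of MoveWaitTime, then resets the timer and flips MoveFlag.
; Move picks the right or forward axis from DummyType, signed by MoveFlag, and applies an unswept world offset of MoveSpeed per frame, unscaled by DeltaSeconds.
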(event EventBeginPlay)

(event Collision|EventActorBeginOverlap
  (params (OtherActor :type Actor%20Object%20Reference)))

(event EventTick
  (params (DeltaSeconds :type Float%20%28single-precision%29))
  (bind _output_get (Variables|Default|SetMoveTotalTime (+ DeltaSeconds (Variables|Default|GetMoveTotalTime))))
  (if (> _output_get (Variables|Default|GetMoveTime))
    (Utilities|FlowControl|Delay (Variables|Default|GetMoveWaitTime))
    (Variables|Default|SetMoveTotalTime 0.0)
    (if (Variables|Default|GetMoveFlag)
      (Variables|Default|SetMoveFlag false)
      (else
        (Variables|Default|SetMoveFlag true)))
    (else
      (CallFunction|Move))))

(event Collision|EventHit
  (params (MyComp :type Primitive%20Component%20Object%20Reference) (Other :type Actor%20Object%20Reference) (OtherComp :type Primitive%20Component%20Object%20Reference) (bSelfMoved :type Boolean) (HitLocation :type Vector :default "0, 0, 0") (HitNormal :type Vector :default "0, 0, 0") (NormalImpulse :type Vector :default "0, 0, 0") (Hit :type Hit%20Result%20Structure%20%28by%20ref%29))
  (Utilities|Casting|CastToBP_FirstPersonProjectile Other)
  (Development|PrintString "Hello"))

(fn ConstructionScript)

(fn Move
  (bind _returnvalue (Transformation|GetActorRightVector))
  (bind _returnvalue_2 (Transformation|GetActorForwardVector))
  (Utilities|FlowControl|Sequence
    (:then_0
      (switch Utilities|FlowControl|Switch|SwitchonEnemyType (Variables|Default|GetDummyType)
        (:NewEnumerator1
          (if (Variables|Default|GetMoveFlag)
            (LocalVariables|SetDirection _returnvalue)
            (else
              (LocalVariables|SetDirection (* _returnvalue -1.0)))))
        (:NewEnumerator2
          (if (Variables|Default|GetMoveFlag)
            (LocalVariables|SetDirection _returnvalue_2)
            (else
              (LocalVariables|SetDirection (* _returnvalue_2 -1.0)))))))
    (:then_1
      (Transformation|AddActorWorldOffset (* (LocalVariables|GetDirection) (Variables|Default|GetMoveSpeed))))))