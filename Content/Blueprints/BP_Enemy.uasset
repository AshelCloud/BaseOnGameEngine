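; BP_Enemy is an enemy pawn that patrols back and forth along a single axis, left/right or forward/back, chosen by EnemyType.
; Tick accumulates time and calls Move, which feeds the actor's right or forward vector, signed by MoveFlag, into AddMovementInput.
; Once MoveTime is exceeded, movement pauses through a Delay of MoveWaitTime, then the timer resets and MoveFlag flips to reverse direction.
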(event EventBeginPlay)

(event Collision|EventActorBeginOverlap
  (params (OtherActor :type Actor%20Object%20Reference)))

(event EventTick
  (params (DeltaSeconds :type Float%20%28single-precision%29))
  (bind _output_get (Variables|Move|SetMoveTotalTime (+ DeltaSeconds (Variables|Move|GetMoveTotalTime))))
  (if (> _output_get (Variables|Move|GetMoveTime))
    (Utilities|FlowControl|Delay (Variables|Move|GetMoveWaitTime))
    (Variables|Move|SetMoveTotalTime 0.0)
    (if (Variables|Move|GetMoveFlag)
      (Variables|Move|SetMoveFlag false)
      (else
        (Variables|Move|SetMoveFlag true)))
    (else
      (CallFunction|Move))))

(fn ConstructionScript)

(fn Move
  (bind _returnvalue (Transformation|GetActorRightVector))
  (bind _returnvalue_2 (Transformation|GetActorForwardVector))
  (Utilities|FlowControl|Sequence
    (:then_0
      (switch Utilities|FlowControl|Switch|SwitchonEnemyType (Variables|Move|GetEnemyType)
        (:NewEnumerator1
          (if (Variables|Move|GetMoveFlag)
            (LocalVariables|SetDirection _returnvalue)
            (else
              (LocalVariables|SetDirection (* _returnvalue -1.0)))))
        (:NewEnumerator2
          (if (Variables|Move|GetMoveFlag)
            (LocalVariables|SetDirection _returnvalue_2)
            (else
              (LocalVariables|SetDirection (* _returnvalue_2 -1.0)))))))
    (:then_1
      (Pawn|Input|AddMovementInput (LocalVariables|GetDirection) (Variables|Move|GetMoveScale) false))))